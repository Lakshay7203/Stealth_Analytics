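; Game manager that tracks a stealth mission run and records analytics events for the third-person level.
; BeginPlay restores the run counter from a save slot and starts a numbered session with timestamped event logging.
; Fail or complete events (also on F/E keys) log the result, save to the slot, export a per-session CSV, then reload the level.
; G prints the CSV text on screen.
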(event `self.ReceiveBeginPlay`
  (`self.EnableInput` (`GameplayStatics.GetPlayerController` 0))
  (`self.CreateAnalysticsSave`)
  (`self.StartSession`))

(event `Key|F`
  (params (Key :type "Key Structure"))
  (:`Pressed`
    (`self.FailMissionEvent`)))

(event `Key|E`
  (params (Key :type "Key Structure"))
  (:`Pressed`
    (`self.CompleteMissionEvent`)))

(event `Key|G`
  (params (Key :type "Key Structure"))
  (:`Pressed`
    (bind _csvtext (`self.BuildCSVText`))
    (`KismetSystemLibrary.PrintString` _csvtext true true (struct :`G` 0.66 :`B` 1.0 :`A` 1.0) 10.0)))

(event `FailMissionEvent`
  (`self.FailMission`)
  (`self.SaveAnalyticsData`)
  (`self.ExportSessionCSV`)
  (`KismetSystemLibrary.Delay` 1.0)
  (`GameplayStatics.OpenLevel` "Lvl_ThirdPerson"))

(event `CompleteMissionEvent`
  (`self.CompleteMission`)
  (`self.SaveAnalyticsData`)
  (`self.ExportSessionCSV`)
  (`KismetSystemLibrary.Delay` 1.0)
  (`GameplayStatics.OpenLevel` "Lvl_ThirdPerson"))

(fn `BuildCSVText`
  (returns (CSVText :type String))
  (set `self.CSVTextLocal` "SessionID,EventType,LevelName,TimeSinceStart,AreaName,GuardID,Result")
  (set `self.CSVTextLocal` (`KismetStringLibrary.Concat_StrStr` (`self.CSVTextLocal`) " \n"))
  (for _array_element (`self.Events`)
    (bind _rowtext (`self.EventToCSVRow` _array_element))
    (set `self.CSVTextLocal` (`KismetStringLibrary.Concat_StrStr` (`self.CSVTextLocal`) _rowtext)))
  (return (`self.CSVTextLocal`)))

(fn `CompleteMission`
  (if (`self.MissionActive?`)
    (set `self.MissionActive?` false)
    (bind _output_get (set `self.MissionResult` "Success"))
    (`self.LogEvent` "Mission Completed" "Exit Zone" "" _output_get)))

(fn `CreateAnalysticsSave`
  (bind _returnvalue (`GameplayStatics.DoesSaveGameExist` "AnalyticsSlot"))
  (if _returnvalue
    (bind _returnvalue_2 (`GameplayStatics.LoadGameFromSlot` "AnalyticsSlot"))
    (bind _asbp_analytics_save_game (cast `/Game/BP_AnalyticsSaveGame` _returnvalue_2))
    (bind _output_get (set `self.AnalysticsSaveRef` _asbp_analytics_save_game))
    (set `self.RunCounter` (`/Game/BP_AnalyticsSaveGame.RunCounter` _output_get))
    (else
      (bind _returnvalue_3 (`GameplayStatics.CreateSaveGameObject` "/Game/BP_AnalyticsSaveGame.BP_AnalyticsSaveGame_C"))
      (bind _asbp_analytics_save_game_2 (cast `/Game/BP_AnalyticsSaveGame` _returnvalue_3))
      (set `self.AnalysticsSaveRef` _asbp_analytics_save_game_2)
      (set `self.RunCounter` 0))))

(fn `EventToCSVRow`
  (params (EventData :type "/Game/ST_GameEvent Structure"))
  (returns (RowText :type String))
  (bind (_sessionid _eventtype _lvlname _timesincestart _areaname _guardid _result) (break `/Game/ST_GameEvent` EventData))
  (return (`KismetStringLibrary.Concat_StrStr` _sessionid "," _eventtype "," _lvlname "," (`KismetStringLibrary.Conv_DoubleToString` _timesincestart) "," _areaname "," _guardid "," _result " \n")))

(fn `ExportSessionCSV`
  (bind _csvtext (`self.BuildCSVText`))
  (bind _returnvalue (`AnalyticsFileLibrary.WriteTextToFile` (`AnalyticsFileLibrary.BuildAnalyticsCSVPath` (`KismetStringLibrary.Concat_StrStr` (`self.SessionID`) ".csv")) _csvtext))
  (if _returnvalue
    (`KismetSystemLibrary.PrintString` "CSV Export Success")
    (else
      (`KismetSystemLibrary.PrintString` "CSV Export Failed"))))

(fn `FailMission`
  ;[0 0 0 0.5] Triggers when the player is caught. Stops the mission timer, sets the result to 'Failed', and sends a final data entry to LogEvent
  (if (`self.MissionActive?`)
    (set `self.MissionActive?` false)
    (bind _output_get (set `self.MissionResult` "Failed"))
    (`self.LogEvent` "Mission Failed" "DetectionZone" "" _output_get)))

(fn `LogEvent`
  (params (eventType :type String) (AreaName :type String) (GuardID :type String) (Result :type String))
  ;[0 0 0 0.5] Calculates time since start ($CurrentTime - SessionStartTime$). Creates a new Event Struct and adds it to the master Events array for later data export
  (bind _returnvalue (`KismetArrayLibrary.Array_Add` (`self.Events`) (make `/Game/ST_GameEvent` (`self.SessionID`) eventType "Lvl_ThirdPerson" (- (`KismetSystemLibrary.GetGameTimeInSeconds`) (`self.SessionStartTime`)) AreaName GuardID Result)))
  (`KismetSystemLibrary.PrintString` (`KismetStringLibrary.Conv_IntToString` _returnvalue)))

(fn `SaveAnalyticsData`
  (bind _analysticssaveref (`self.AnalysticsSaveRef`))
  (`/Engine/EditorBlueprintResources/StandardMacros.IsValid` _analysticssaveref
    (:`Is Valid`
      (set `/Game/BP_AnalyticsSaveGame.Events` (`self.Events`) _analysticssaveref)
      (set `/Game/BP_AnalyticsSaveGame.RunCounter` (`self.RunCounter`) _analysticssaveref)
      (bind _returnvalue (`GameplayStatics.SaveGameToSlot` _analysticssaveref "AnalyticsSlot"))
      (if _returnvalue
        (`KismetSystemLibrary.PrintString` "Save Sucess")
        (else
          (`KismetSystemLibrary.PrintString` "Save Failed"))))))

(fn `StartSession`
  ;[0 0 0 0.5] Initializes the game session. Sets mission to 'InProgress' and records the GameTime to use as the $T=0$ baseline for analytics.
  (bind _output_get (set `self.RunCounter` (+ (`self.RunCounter`) 1)))
  (set `self.SessionID` (`KismetStringLibrary.Concat_StrStr` "Run_" (`KismetStringLibrary.Conv_IntToString` _output_get)))
  (set `self.SessionStartTime` (`KismetSystemLibrary.GetGameTimeInSeconds`))
  (`KismetArrayLibrary.Array_Clear` (`self.Events`))
  (set `self.MissionActive?` true)
  (bind _output_get_2 (set `self.MissionResult` "InProgress"))
  (`self.LogEvent` "SessionStart" "StartArea" "" _output_get_2))

(fn `UserConstructionScript`)