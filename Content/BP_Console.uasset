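; BP_Console is an objective actor that the player completes by walking into its PickupTrigger.
; On the first overlap by BP_ThirdPersonCharacter, guarded by a DoOnce, it finds BP_GameManager and logs an ObjectiveCompleted event with its AreaName and ObjectiveID.
; It then increments the manager's ObjectiveCompleted counter, prints the new count and destroys itself.
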(event `self.PickupTrigger.OnComponentBeginOverlap`
  (params (OverlappedComponent :type "PrimitiveComponent Object Reference") (OtherActor :type "Actor Object Reference") (OtherComp :type "PrimitiveComponent Object Reference") (OtherBodyIndex :type Integer) (bFromSweep :type Boolean) (SweepResult :type "HitResult Structure (by ref)"))
  (cast `/Game/ThirdPerson/Blueprints/BP_ThirdPersonCharacter` OtherActor)
  (`/Engine/EditorBlueprintResources/StandardMacros.DoOnce` false
    (:`Completed`
      (bind _returnvalue (`GameplayStatics.GetActorOfClass` "/Game/BP_GameManager.BP_GameManager_C"))
      (`/Game/BP_GameManager.LogEvent` _returnvalue "ObjectiveCompleted" (`self.AreaName`) "" (`self.ObjectiveID`))
      (bind _output_get (set `/Game/BP_GameManager.ObjectiveCompleted` (+ (`/Game/BP_GameManager.ObjectiveCompleted` _returnvalue) 1) _returnvalue))
      (`KismetSystemLibrary.PrintString` (`KismetStringLibrary.Conv_IntToString` _output_get))
      (`self.K2_DestroyActor`))))

(fn `UserConstructionScript`)